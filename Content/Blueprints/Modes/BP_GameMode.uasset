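; BP_GameMode is the game mode that sets up menu levels and handles the player's game over.
; On BeginPlay it checks the level name, and on MainMenu or EndGame shows that screen's widget, enables the cursor and destroys the player character.
; Its EndGame event shows a death menu, passes it the current level name, enables the cursor and blocks look input.
; It also holds a CanPlayerLeave flag with a getter and a one-way setter.
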(event Custom|EndGame
  (bind _returnvalue (Game|GetPlayerController 0))
  (bind _returnvalue_2 (UserInterface|CreateWidget "/Game/UI/BPW_DeathMenu.BPW_DeathMenu_C"))
  (bind _output_get (Variables|Default|SetDeathUI _returnvalue_2))
  (UserInterface|Viewport|AddtoViewport _output_get 0)
  (bind _returnvalue_3 (Game|GetCurrentLevelName true))
  (Development|PrintString _returnvalue_3)
  (Default|SetLevelName (Variables|Default|GetDeathUI) (Utilities|String|StringToName _returnvalue_3))
  (Variables|/Script/Engine.PlayerController|SetbShowMouseCursor _returnvalue true)
  (Input|SetIgnoreLookInput _returnvalue true))

(event EventBeginPlay
  (Utilities|FlowControl|Sequence
    (:then_0
      (bind _returnvalue (Game|GetCurrentLevelName true))
      (if (Utilities|Enum|Equal(Enum) _returnvalue "MainMenu")
        (bind _returnvalue_2 (UserInterface|CreateWidget "/Game/UI/MainMenu.MainMenu_C"))
        (UserInterface|Viewport|AddtoViewport _returnvalue_2 0)
        (Variables|/Script/Engine.PlayerController|SetbShowMouseCursor (Game|GetPlayerController 0) true)
        (Actor|DestroyActor (Game|GetPlayerCharacter 0))))
    (:then_1
      (bind _returnvalue_3 (Game|GetCurrentLevelName true))
      (if (Utilities|Enum|Equal(Enum) _returnvalue_3 "EndGame")
        (bind _returnvalue_4 (UserInterface|CreateWidget "/Game/UI/UI_End.UI_End_C"))
        (UserInterface|Viewport|AddtoViewport _returnvalue_4 0)
        (Variables|/Script/Engine.PlayerController|SetbShowMouseCursor (Game|GetPlayerController 0) true)
        (Actor|DestroyActor (Game|GetPlayerCharacter 0))))))

(fn ConstructionScript)

(fn CanLeavetheArea
  (return (Variables|Default|GetCanPlayerLeave)))

(fn SetPlayerLeave
  (Variables|Default|SetCanPlayerLeave true))