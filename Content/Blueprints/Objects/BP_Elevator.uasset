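; BP_Elevator is an interactable elevator whose two doors slide apart, with an optional dialogue shown at BeginPlay.
; When ShouldDialogue is set, it creates the dialogue widget, passes itself in, blocks interaction and switches to UI-only input.
; DialogueFinished removes the widget, re-enables interaction and restores game-only input.
; Interact, gated by CanInteract, plays the OpenDoors timeline to lerp both doors' relative X positions.
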(event Custom|DialogueFinished
  (Widget|RemovefromParent (Variables|Default|GetDialogue))
  (Variables|Default|SetCanInteract true)
  (Input|SetInputModeGameOnly (Game|GetPlayerController 0) false))

(event EventBeginPlay
  (|CallParentFunction)
  (if (Variables|Default|GetShouldDialogue)
    (bind _returnvalue (UserInterface|CreateWidget "/Game/UI/UiDialogue.UiDialogue_C"))
    (bind _output_get (Variables|Default|SetDialogue _returnvalue))
    (UserInterface|Viewport|AddtoViewport _output_get 0)
    (Default|SetDoor _output_get self)
    (Utilities|IsValid _output_get
      (:Is%20Valid
        (Variables|Default|SetCanInteract false)
        (Input|SetInputModeUIOnly (Game|GetPlayerController 0) (Variables|Default|GetDialogue) "LockOnCapture" false))
      (:Is%20Not%20Valid
        (Variables|Default|SetCanInteract true)))))

(event Collision|EventActorBeginOverlap
  (params (OtherActor :type Actor%20Object%20Reference))
  (|CallParentFunction OtherActor) ; This node is disabled and will not be called.\nDrag off pins to build functionality.
)

(event EventTick
  (params (DeltaSeconds :type Float%20%28single-precision%29))
  (|CallParentFunction DeltaSeconds) ; This node is disabled and will not be called.\nDrag off pins to build functionality.
)

(event EventInteract
  (if (Variables|Default|GetCanInteract)
    (Development|PrintString "Hello")
    (bind _alpha (Timeline|OpenDoors Play)
      (:Update
        (Transformation|SetRelativeLocation (Variables|Default|GetDoor) (Math|Vector|MakeVector (Math|Float|Lerp -78.0 -4.0 _alpha) 0.0 0.0) false false)
        (Transformation|SetRelativeLocation (Variables|Default|GetDoor1) (Math|Vector|MakeVector (Math|Float|Lerp -148.0 -222.0 _alpha) 0.0 0.0) false false)))))

(fn ConstructionScript
  (|CallParentFunction))