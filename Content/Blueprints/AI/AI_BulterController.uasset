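; AI controller for the butler that runs its behavior tree and reacts to perceiving the player character.
; On BeginPlay it starts the tree and saves the pawn's starting location to the blackboard.
; Sensing a BP_Character sets the visible, pursuing and surprised-animation flags.
; Losing the character clears only the visibility flag, leaving the other two untouched by the controller.
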(event OnTargetPerceptionUpdated(AIPerception)
  (params (Actor :type Actor%20Object%20Reference) (Stimulus :type AI%20Stimulus%20Structure))
  (Utilities|Casting|CastToBP_Character Actor)
  (if (.bSuccessfullySensed (Utilities|Struct|BreakAIStimulus Stimulus))
    (AI|Components|Blackboard|SetValueasBool (AI|GetBlackboard 0) (Utilities|Name|MakeLiteralName "CanSeeThePlayer") true)
    (AI|Components|Blackboard|SetValueasBool (AI|GetBlackboard 0) (Utilities|Name|MakeLiteralName "IsPursuing") true)
    (AI|Components|Blackboard|SetValueasBool (AI|GetBlackboard 0) (Utilities|Name|MakeLiteralName "PlayAnimSurprised") true)
    (else
      (Development|PrintString "palyer not set")
      (AI|Components|Blackboard|SetValueasBool (AI|GetBlackboard 0) (Utilities|Name|MakeLiteralName "CanSeeThePlayer") false))))

(event EventBeginPlay
  (AI|RunBehaviorTree "/Game/Blueprints/AI/AI_ButlerController.AI_ButlerController")
  (AI|Components|Blackboard|SetValueasVector (AI|GetBlackboard 0) (Utilities|Name|MakeLiteralName "InitialLocation") (Transformation|GetActorLocation (Pawn|GetControlledPawn))))

(fn ConstructionScript)